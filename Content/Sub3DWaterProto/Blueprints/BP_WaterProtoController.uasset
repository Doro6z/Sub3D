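; Player controller for the 3D water prototype, handling look input and a debug key for disturbing room water.
; IA_Look feeds yaw and inverted pitch input to the first player pawn.
; Pressing E traces from the view through SubInteraction and injects a fixed force and radius at the hit point into the hit actor's RoomWaterRenderer component.
; The same press prints the hit actor's name and draws a brief debug box there.
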(event Input|EnhancedActionEvents|EnhancedInputActionIA_Look
  (params (ActionValue :type Vector%202D%20Structure) (ElapsedSeconds :type Float%20%28double-precision%29) (TriggeredSeconds :type Float%20%28double-precision%29) (InputAction :type Input%20Action%20Object%20Reference :default "/Game/Sub3D/Input/ONFOOT/IA_Look.IA_Look"))
  (bind (_x _y) (Math|Vector2D|BreakVector2D ActionValue))
  (bind _returnvalue (Game|Player|GetPlayerPawn 0))
  (Utilities|IsValid (Game|Player|GetPlayerPawn 0)
    (:Is%20Valid
      (Pawn|Input|AddControllerYawInput _returnvalue _x)
      (Pawn|Input|AddControllerPitchInput _returnvalue (* _y -1.0)))))

(event EventBeginPlay)

(event Collision|EventActorBeginOverlap
  (params (OtherActor :type Actor%20Object%20Reference)))

(event EventTick
  (params (DeltaSeconds :type Float%20%28single-precision%29)))

(event Input|KeyboardEvents|DebugKeyR
  (params (Key :type Key%20Structure :default "None") (ActionValue :type Input%20Action%20Value%20Structure)))

(event Input|KeyboardEvents|DebugKeyE
  (params (Key :type Key%20Structure :default "None") (ActionValue :type Input%20Action%20Value%20Structure))
  (bind _subinteraction (Variables|Default|GetSubInteraction))
  (bind _outhit (Class|SubInteractionComponent|TracefromView _subinteraction))
  (:Pressed
    (Development|PrintString (Utilities|GetDisplayName (.hitactor _outhit)))
    (Class|RoomWaterRenderer|InjectatWorldPoint (Actor|GetComponentbyClass (.hitactor _outhit) "/Script/Sub3DWaterProto.RoomWaterRenderer") (.location _outhit) 5.0 3e+01)
    (Rendering|Debug|DrawDebugBox (.location _outhit) "15.000000,15.000000,15.000000" "(R=1.000000,G=0.000000,B=0.058713,A=1.000000)" "0, 0, 0" 2.0 2.0)))

(fn ConstructionScript)