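; BP_SubmarineCrew is the submarine crew player Blueprint, binding Enhanced Input for interacting and repairing.
; Interact and Repair inputs forward to InteractionComponent, which handles primary interaction, tool action begin and end, and repair of the focused target when the press starts.
; A custom event plays a hull-impact world camera shake at the actor's location, but its looping timer is disconnected, so nothing in this graph triggers it.
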(event Custom|CustomEvent
  (Camera|PlayWorldCameraShake "/Game/Sub3D/Proto04C/Feedback/CS_HullImpact.CS_HullImpact_C" (Transformation|GetActorLocation) 5e+02 5e+02))

(event Input|EnhancedActionEvents|EnhancedInputActionIA_Repair
  (params (ActionValue :type Boolean) (ElapsedSeconds :type Float%20%28double-precision%29) (TriggeredSeconds :type Float%20%28double-precision%29) (InputAction :type Input%20Action%20Object%20Reference :default "/Game/Sub3D/Input/ONFOOT/IA_Repair.IA_Repair"))
  (bind _interactioncomponent (Variables|Default|GetInteractionComponent))
  (:Started
    (Class|SubInteractionComponent|BeginToolAction _interactioncomponent)
    (Class|SubInteractionComponent|TryRepairFocusedTarget _interactioncomponent 2e+01 3e+01))
  (:Completed
    (Class|SubInteractionComponent|EndToolAction (Variables|Default|GetInteractionComponent))))

(event Input|EnhancedActionEvents|EnhancedInputActionIA_Interact
  (params (ActionValue :type Boolean) (ElapsedSeconds :type Float%20%28double-precision%29) (TriggeredSeconds :type Float%20%28double-precision%29) (InputAction :type Input%20Action%20Object%20Reference :default "/Game/Sub3D/Input/ONFOOT/IA_Interact.IA_Interact"))
  (:Started
    (Class|SubInteractionComponent|TryPrimaryInteract (Variables|Default|GetInteractionComponent))))

(event EventBeginPlay)

(fn ConstructionScript)