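; Player controller for submarine crew, switching between on-foot, helm driving and station UI control modes.
; ApplyControlMode runs on mode changes, swapping Enhanced Input contexts, input mode, cursor and station widgets locally.
; Helm, turret and sonar ping inputs go to server routing calls, including hold-to-steer mouse input that restores the cursor position.
; It also handles movement, radar toggle, sonar-lean camera FOV, station exit and departure from boarding.
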(event Custom|PCRequest%20Exit%20Station
  ;[0.15 0.15 0.15 0.5] Exit Station
  (Class|SubPlayerController|ServerExitStation))

(event Custom|PC_BeginDeparture
  (bind _asbp_sub_gamemode (Utilities|Casting|CastToBP_SubGamemode (Game|GetGameMode)))
  (if (Utilities|Enum|Equal(Enum) (Variables|/Script/Sub3D.SubGameMode|GetRunPhase _asbp_sub_gamemode) "Boarding")
    (Class|SubGameMode|BeginDeparture _asbp_sub_gamemode)))

(event Input|EnhancedActionEvents|EnhancedInputActionIA_Thrust
  (params (ActionValue :type Float%20%28double-precision%29) (ElapsedSeconds :type Float%20%28double-precision%29) (TriggeredSeconds :type Float%20%28double-precision%29) (InputAction :type Input%20Action%20Object%20Reference :default "/Game/Sub3D/Input/HELM/IA_Thrust.IA_Thrust"))
  ;[0.0405 0.07497 0.15 0.5] Sub Helm - Pilot
  (:Triggered
    (if (Utilities|Enum|Equal(Enum) (Variables|Default|GetCurrentControlMode) "HelmDriving")
      (Class|SubPlayerController|ServerRouteHelmThrust ActionValue)))
  (:Completed
    (if (Utilities|Enum|Equal(Enum) (Variables|Default|GetCurrentControlMode) "HelmDriving")
      (Class|SubPlayerController|ServerRouteHelmThrust 0.0))))

(event Input|EnhancedActionEvents|EnhancedInputActionIA_Move
  (params (ActionValue :type Vector%202D%20Structure) (ElapsedSeconds :type Float%20%28double-precision%29) (TriggeredSeconds :type Float%20%28double-precision%29) (InputAction :type Input%20Action%20Object%20Reference :default "/Game/Sub3D/Input/ONFOOT/IA_Move.IA_Move"))
  ;[0.15 0.15 0.15 0.5] OnFoot
  (|OnFootIA_Move ActionValue))

(event Input|EnhancedActionEvents|EnhancedInputActionIA_SonarPing
  (params (ActionValue :type Boolean) (ElapsedSeconds :type Float%20%28double-precision%29) (TriggeredSeconds :type Float%20%28double-precision%29) (InputAction :type Input%20Action%20Object%20Reference :default "/Game/Sub3D/Input/HELM/IA_SonarPing.IA_SonarPing"))
  ;[0.0405 0.07497 0.15 0.5] Sub Helm - Pilot
  ;;[0.04739 0.07031 0.15 0.5] Sonar
  (:Started
    (Class|SubPlayerController|ServerSetSonarPingHeld true))
  (:Canceled
    (Class|SubPlayerController|ServerSetSonarPingHeld false :!label _label))
  (:Completed
    (goto _label)))

(event Input|EnhancedActionEvents|EnhancedInputActionIA_SonarLean
  (params (ActionValue :type Boolean) (ElapsedSeconds :type Float%20%28double-precision%29) (TriggeredSeconds :type Float%20%28double-precision%29) (InputAction :type Input%20Action%20Object%20Reference :default "/Game/Sub3D/Input/HELM/IA_SonarLean.IA_SonarLean"))
  ;[0.0405 0.07497 0.15 0.5] Sub Helm - Pilot
  ;;[0.04739 0.07031 0.15 0.5] Sonar
  (:Started
    (Class|SubPlayerController|SetSonarLeanActive true))
  (:Canceled
    (Class|SubPlayerController|SetSonarLeanActive false :!label _label))
  (:Completed
    (goto _label)))

(event Input|EnhancedActionEvents|EnhancedInputActionIA_Look
  (params (ActionValue :type Vector%202D%20Structure) (ElapsedSeconds :type Float%20%28double-precision%29) (TriggeredSeconds :type Float%20%28double-precision%29) (InputAction :type Input%20Action%20Object%20Reference :default "/Game/Sub3D/Input/ONFOOT/IA_Look.IA_Look"))
  (bind (_x _y) (Math|Vector2D|BreakVector2D ActionValue))
  (bind _returnvalue (Game|Player|GetPlayerPawn 0))
  ;[0.15 0.15 0.15 0.5] OnFoot
  (Pawn|Input|AddControllerYawInput _returnvalue _x)
  (Pawn|Input|AddControllerPitchInput _returnvalue (* _y -1.0)))

(event Input|EnhancedActionEvents|EnhancedInputActionIA_DivePlane
  (params (ActionValue :type Float%20%28double-precision%29) (ElapsedSeconds :type Float%20%28double-precision%29) (TriggeredSeconds :type Float%20%28double-precision%29) (InputAction :type Input%20Action%20Object%20Reference :default "/Game/Sub3D/Input/HELM/IA_DivePlane.IA_DivePlane"))
  ;[0.0405 0.07497 0.15 0.5] Sub Helm - Pilot
  (:Triggered
    (if (Utilities|Enum|Equal(Enum) (Variables|Default|GetCurrentControlMode) "HelmDriving")
      (Class|SubPlayerController|ServerRouteHelmDive ActionValue)))
  (:Completed
    (if (Utilities|Enum|Equal(Enum) (Variables|Default|GetCurrentControlMode) "HelmDriving")
      (Class|SubPlayerController|ServerRouteHelmDive 0.0))))

(event Input|EnhancedActionEvents|EnhancedInputActionIA_ExitStation
  (params (ActionValue :type Boolean) (ElapsedSeconds :type Float%20%28double-precision%29) (TriggeredSeconds :type Float%20%28double-precision%29) (InputAction :type Input%20Action%20Object%20Reference :default "/Game/Sub3D/Input/IA_ExitStation.IA_ExitStation"))
  ;[0.15 0.15 0.15 0.5] Exit Station
  (if (Utilities|Enum|NotEqual(Enum) (Variables|Default|GetCurrentControlMode) "OnFoot")
    (CallFunction|PCRequestExitStation)))

(event Input|EnhancedActionEvents|EnhancedInputActionIA_RadarToggle
  (params (ActionValue :type Boolean) (ElapsedSeconds :type Float%20%28double-precision%29) (TriggeredSeconds :type Float%20%28double-precision%29) (InputAction :type Input%20Action%20Object%20Reference :default "/Game/Sub3D/Input/HELM/IA_RadarToggle.IA_RadarToggle"))
  ;[0.0405 0.07497 0.15 0.5] Sub Helm - Pilot
  ;;[0.15 0.15 0.15 0.5] Radar Input
  (:Started
    (bind _radarwidgetref (Variables|Default|GetRadarWidgetRef)
      (:then
        (if (Utilities|Enum|Equal(Enum) (Widget|GetVisibility _radarwidgetref) "Visible")
          (Variables|/Script/UMG.Widget|SetVisibility (Variables|Default|GetRadarWidgetRef) "Collapsed")
          (else
            (Variables|/Script/UMG.Widget|SetVisibility (Variables|Default|GetRadarWidgetRef) "Visible"))))
      (:else
        (bind _returnvalue (UserInterface|CreateWidget "/Game/Sub3D/UI/WBP_SubRadar.WBP_SubRadar_C"))
        (bind _output_get (Variables|Default|SetRadarWidgetRef _returnvalue))
        (UserInterface|Viewport|AddtoViewport _output_get 0)))))

(event Input|EnhancedActionEvents|EnhancedInputActionIA_HelmDirectInputHold
  (params (ActionValue :type Boolean) (ElapsedSeconds :type Float%20%28double-precision%29) (TriggeredSeconds :type Float%20%28double-precision%29) (InputAction :type Input%20Action%20Object%20Reference :default "/Game/Sub3D/Input/HELM/IA_HelmDirectInputHold.IA_HelmDirectInputHold"))
  ;[0.0405 0.07497 0.15 0.5] Sub Helm - Pilot
  (:Started
    (Variables|Default|SetbDirectHelmInputActive true)
    (Input|SetInputModeGameOnly self false)
    (CallFunction|ToggleOffHelmDirectInputMouse))
  (:Canceled
    (Variables|Default|SetbDirectHelmInputActive false :!label _label)
    (Input|SetInputModeGameandUI self 0 "DoNotLock" false false)
    (CallFunction|ToggleBackHelmDirectInputMouse))
  (:Completed
    (goto _label)))

(event Input|EnhancedActionEvents|EnhancedInputActionIA_FireTurret
  (params (ActionValue :type Boolean) (ElapsedSeconds :type Float%20%28double-precision%29) (TriggeredSeconds :type Float%20%28double-precision%29) (InputAction :type Input%20Action%20Object%20Reference :default "/Game/Sub3D/Input/IA_FireTurret.IA_FireTurret"))
  ;[0.0405 0.07497 0.15 0.5] Sub Helm - Pilot
  ;;[0.15 0.15 0.15 0.5] IA FireTurret
  (:Triggered
    (Class|SubPlayerController|ServerRouteTurretFire true))
  (:Completed
    (Class|SubPlayerController|ServerRouteTurretFire false)))

(event Input|EnhancedActionEvents|EnhancedInputActionIA_Rudder
  (params (ActionValue :type Float%20%28double-precision%29) (ElapsedSeconds :type Float%20%28double-precision%29) (TriggeredSeconds :type Float%20%28double-precision%29) (InputAction :type Input%20Action%20Object%20Reference :default "/Game/Sub3D/Input/HELM/IA_Rudder.IA_Rudder"))
  ;[0.0405 0.07497 0.15 0.5] Sub Helm - Pilot
  (:Triggered
    (if (Utilities|Enum|Equal(Enum) (Variables|Default|GetCurrentControlMode) "HelmDriving")
      (Class|SubPlayerController|ServerRouteHelmSteer ActionValue)))
  (:Completed
    (if (Utilities|Enum|Equal(Enum) (Variables|Default|GetCurrentControlMode) "HelmDriving")
      (Class|SubPlayerController|ServerRouteHelmSteer 0.0))))

(event Input|EnhancedActionEvents|EnhancedInputActionIA_HelmMouseDirect
  (params (ActionValue :type Vector%202D%20Structure) (ElapsedSeconds :type Float%20%28double-precision%29) (TriggeredSeconds :type Float%20%28double-precision%29) (InputAction :type Input%20Action%20Object%20Reference :default "/Game/Sub3D/Input/HELM/IA_HelmMouseDirect.IA_HelmMouseDirect"))
  (bind (_x _y) (Math|Vector2D|BreakVector2D ActionValue))
  ;[0.0405 0.07497 0.15 0.5] Sub Helm - Pilot
  (if (Variables|Default|GetbDirectHelmInputActive)
    (Class|SubPlayerController|ServerRouteHelmDive (* (Variables|Default|GetbDirectHelmInputMouseSensitivityY) _y))
    (if (Variables|Default|GetbDirectHelmYawEnabled)
      (Class|SubPlayerController|ServerRouteHelmDive (* (Variables|Default|GetbDirectHelmInputMouseSensitivityX) _x)))))

(event EventBeginPlay
  (CallFunction|ApplyControlMode (Variables|Default|GetCurrentControlMode) "None"))

(event EventTick
  (params (DeltaSeconds :type Float%20%28single-precision%29)))

(event EventOnControlModeChanged
  (params (NewMode :type ECrewControlMode%20Enum :default "OnFoot") (StationType :type ESubStationType%20Enum :default "None"))
  ;[0.06816 0.01937 0.08854] Event BP OnControlModeChanged
  (CallFunction|ApplyControlMode NewMode StationType))

(event EventOnSonarLeanChanged
  (params (bActive :type Boolean))
  ;[0.0405 0.07497 0.15 0.5] Sub Helm - Pilot
  (bind _asbp_submarine_crew (Utilities|Casting|CastToBP_SubmarineCrew (Game|Player|GetPlayerPawn 0)))
  (if bActive
    (Camera|SetFieldOfView (Variables|/Game/Sub3D/Blueprint/PlayerBP/BP_SubmarineCrew.BP_SubmarineCrew_C|GetTPSCamera _asbp_submarine_crew) 6e+01)
    (else
      (Camera|SetFieldOfView (Variables|/Game/Sub3D/Blueprint/PlayerBP/BP_SubmarineCrew.BP_SubmarineCrew_C|GetTPSCamera _asbp_submarine_crew) 9e+01))))

(fn ConstructionScript)

(fn ApplyControlMode
  (params (Mode :type ECrewControlMode%20Enum :default "OnFoot") (StationType :type ESubStationType%20Enum :default "None"))
  (bind _returnvalue (PlayerController|LocalPlayerSubsystems|GetEnhancedInputLocalPlayerSubsystem))
  (LocalVariables|SetNewControlMode Mode)
  (LocalVariables|SetNewStationType StationType)
  (if (Pawn|IsLocalController)
    ;[0.15 0.15 0.15 0.5] Clear IMC
    (Utilities|FlowControl|Sequence
      (:then_0
        (Input|RemoveMappingContext _returnvalue (Variables|Default|GetIMC_OnFoot) "(bIgnoreAllPressedKeysUntilRelease=True,bForceImmediately=False,bNotifyUserSettings=False)"))
      (:then_1
        (Input|RemoveMappingContext _returnvalue (Variables|Default|GetIMC_Helm) "(bIgnoreAllPressedKeysUntilRelease=True,bForceImmediately=False,bNotifyUserSettings=False)"))
      (:then_2
        (Input|RemoveMappingContext _returnvalue (Variables|Default|GetIMC_StationUI) "(bIgnoreAllPressedKeysUntilRelease=True,bForceImmediately=False,bNotifyUserSettings=False)")
        ;[0.401 0.3604 0.2569 0.5 65] Debug
        (Development|PrintString (Utilities|String|Append "BPVar(VarName=\"NewLocalVar\",VarGuid=A25BDC214A354207066B2CA3D1D44EA9,VarType=(PinCategory=\"byte\",PinSubCategory=\"\",PinSubCategoryObject=\"/Script/CoreUObject.Enum'/Script/Sub3D.ECrewControlMode'\",PinSubCategoryMemberReference=(MemberParent=None,MemberName=\"\",MemberGuid=00000000000000000000000000000000),PinValueType=(TerminalCategory=\"\",TerminalSubCategory=\"\",TerminalSubCategoryObject=None,bTerminalIsConst=False,bTerminalIsWeakPointer=False,bTerminalIsUObjectWrapper=False),ContainerType=None,bIsReference=False,bIsConst=False,bIsWeakPointer=False,bIsUObjectWrapper=False,bSerializeAsSinglePrecisionFloat=False),FriendlyName=\"New Local Var\",Category=NSLOCTEXT(\"KismetSchema\", \"Default\", \"Default\"),PropertyFlags=5,RepNotifyFunc=\"\",ReplicationCondition=COND_None,MetaDataArray=,DefaultValue=\"OnFoot\")" (Utilities|String|EnumtoString (LocalVariables|GetNewControlMode))) false)
        ;[0.15 0.15 0.15 0.5] Clear Widget
        (CallFunction|RemoveAllStationWidgets)
        ;[0.1301 0.1329 0.04971] NewControlMode
        (switch Utilities|FlowControl|Switch|SwitchonECrewControlMode (LocalVariables|GetNewControlMode)
          (:OnFoot
            ;[0.1304 0.6957 0.07826 0.5] Control On Foot
            (Input|SetInputModeGameOnly self false)
            (Variables|Default|SetbShowMouseCursor false)
            (Input|AddMappingContext (PlayerController|LocalPlayerSubsystems|GetEnhancedInputLocalPlayerSubsystem) (Variables|Default|GetIMC_OnFoot) 0 "(bIgnoreAllPressedKeysUntilRelease=True,bForceImmediately=False,bNotifyUserSettings=False)")
            (Game|Player|SetViewTargetwithBlend (Pawn|GetControlledPawn) 0.0 "VTBlend_Linear" 0.0 false)
            (Variables|Default|SetbDirectHelmInputActive false))
          (:HelmDriving
            ;[0.0405 0.07497 0.15 0.5] Control Helm
            (Input|SetInputModeGameandUI self 0 "DoNotLock" false false)
            (Variables|Default|SetbShowMouseCursor true)
            (Input|AddMappingContext (PlayerController|LocalPlayerSubsystems|GetEnhancedInputLocalPlayerSubsystem) (Variables|Default|GetIMC_Helm) 1 "(bIgnoreAllPressedKeysUntilRelease=True,bForceImmediately=False,bNotifyUserSettings=False)")
            (bind _helmwidgetref (Variables|Default|GetHelmWidgetRef)
              (:then
                (UserInterface|Viewport|AddtoViewport _helmwidgetref 0))
              (:else
                (bind _returnvalue_2 (UserInterface|CreateWidget "/Game/Sub3D/UI/WBP_SubHelm.WBP_SubHelm_C"))
                (UserInterface|Viewport|AddtoViewport _returnvalue_2 0)
                (bind _output_get (Variables|Default|SetHelmWidgetRef _returnvalue_2))))
            (Variables|Default|SetbDirectHelmInputActive false)
            (Class|SubHelmWidget|InitforCrew _output_get (.AsSub%20Crew%20Character (Utilities|Casting|CastToSubCrewCharacter (Pawn|GetControlledPawn)))))
          (:StationUI
            ;[1 0.1684 0 0.3043] Control Station UI
            (Input|SetInputModeGameandUI self 0 "DoNotLock" true false)
            (Variables|Default|SetbShowMouseCursor true)
            (Input|AddMappingContext (PlayerController|LocalPlayerSubsystems|GetEnhancedInputLocalPlayerSubsystem) (Variables|Default|GetIMC_StationUI) 1 "(bIgnoreAllPressedKeysUntilRelease=True,bForceImmediately=False,bNotifyUserSettings=False)")
            (switch Utilities|FlowControl|Switch|SwitchonESubStationType (LocalVariables|GetNewStationType)
              (:Engine
                (bind _returnvalue_3 (UserInterface|CreateWidget "/Game/Sub3D/UI/WBP_SubEngine.WBP_SubEngine_C"))
                (UserInterface|Viewport|AddtoViewport _returnvalue_3 0)
                (Variables|Default|SetEngineWidgetRef _returnvalue_3))
              (:Ballast
                (bind _returnvalue_4 (UserInterface|CreateWidget "/Game/Sub3D/UI/WBP_SubBallast.WBP_SubBallast_C"))
                (UserInterface|Viewport|AddtoViewport _returnvalue_4 0)
                (Variables|Default|SetBallastWidgetRef _returnvalue_4))
              (:Turret
                (bind _returnvalue_5 (UserInterface|CreateWidget "/Game/Sub3D/UI/WBP_SubTurret.WBP_SubTurret_C"))
                (UserInterface|Viewport|AddtoViewport _returnvalue_5 0)
                (Variables|Default|SetTurretWidgetRef _returnvalue_5)))))))))

(fn RemoveAllStationWidgets
  (Utilities|FlowControl|Sequence
    (:then_0
      ;[0.15 0.15 0.15 0.5] HelmWidget
      (bind _helmwidgetref (Variables|Default|GetHelmWidgetRef)
        (:then
          (Widget|RemovefromParent _helmwidgetref)
          (Variables|Default|SetHelmWidgetRef 0))
        (:else)))
    (:then_1
      ;[0.15 0.15 0.15 0.5] EngineWidget
      (bind _enginewidgetref (Variables|Default|GetEngineWidgetRef)
        (:then
          (Widget|RemovefromParent _enginewidgetref)
          (Variables|Default|SetEngineWidgetRef 0))
        (:else)))
    (:then_2
      ;[0.15 0.15 0.15 0.5] TurretWidget
      (bind _turretwidgetref (Variables|Default|GetTurretWidgetRef)
        (:then
          (Widget|RemovefromParent _turretwidgetref)
          (Variables|Default|SetTurretWidgetRef 0))
        (:else)))
    (:then_3
      ;[0.15 0.15 0.15 0.5] BallastWidget
      (bind _ballastwidgetref (Variables|Default|GetBallastWidgetRef)
        (:then
          (Widget|RemovefromParent _ballastwidgetref)
          (Variables|Default|SetBallastWidgetRef 0))
        (:else)))))

(fn CreateStationWidgetfromType
  (params (StationType :type ESubStationType%20Enum :default "None"))
  (CallFunction|RemoveAllStationWidgets)
  (switch Utilities|FlowControl|Switch|SwitchonESubStationType StationType
    (:Helm
      (bind _helmwidgetref (Variables|Default|GetHelmWidgetRef)
        (:then
          (if (not (UserInterface|Viewport|IsinViewport _helmwidgetref))
            (UserInterface|Viewport|AddtoViewport _helmwidgetref 0)))
        (:else
          (bind _returnvalue (UserInterface|CreateWidget "/Game/Sub3D/UI/WBP_SubHelm.WBP_SubHelm_C"))
          (bind _output_get (Variables|Default|SetHelmWidgetRef _returnvalue))
          (UserInterface|Viewport|AddtoViewport _output_get 0))))
    (:Engine
      (bind _enginewidgetref (Variables|Default|GetEngineWidgetRef)
        (:then
          (if (not (UserInterface|Viewport|IsinViewport _enginewidgetref))
            (UserInterface|Viewport|AddtoViewport _enginewidgetref 0)))
        (:else
          (bind _returnvalue_2 (UserInterface|CreateWidget "/Game/Sub3D/UI/WBP_SubEngine.WBP_SubEngine_C"))
          (bind _output_get_2 (Variables|Default|SetEngineWidgetRef _returnvalue_2))
          (UserInterface|Viewport|AddtoViewport _output_get_2 0))))
    (:Ballast
      (bind _ballastwidgetref (Variables|Default|GetBallastWidgetRef)
        (:then
          (if (not (UserInterface|Viewport|IsinViewport _ballastwidgetref))
            (UserInterface|Viewport|AddtoViewport _ballastwidgetref 0)))
        (:else
          (bind _returnvalue_3 (UserInterface|CreateWidget "/Game/Sub3D/UI/WBP_SubBallast.WBP_SubBallast_C"))
          (bind _output_get_3 (Variables|Default|SetBallastWidgetRef _returnvalue_3))
          (UserInterface|Viewport|AddtoViewport _output_get_3 0))))
    (:Turret
      (bind _turretwidgetref (Variables|Default|GetTurretWidgetRef)
        (:then
          (if (not (UserInterface|Viewport|IsinViewport _turretwidgetref))
            (UserInterface|Viewport|AddtoViewport _turretwidgetref 0)))
        (:else
          (bind _returnvalue_4 (UserInterface|CreateWidget "/Game/Sub3D/UI/WBP_SubTurret.WBP_SubTurret_C"))
          (bind _output_get_4 (Variables|Default|SetTurretWidgetRef _returnvalue_4))
          (UserInterface|Viewport|AddtoViewport _output_get_4 0))))))

(fn ToggleOffHelmDirectInputMouse
  (bind (_locationx _locationy) (Game|Player|GetMousePosition))
  (Variables|Default|SetbShowMouseCursor false)
  (Variables|Default|SetDirectHelMouseLocationCache (Math|Vector2D|MakeVector2D _locationx _locationy)))

(fn ToggleBackHelmDirectInputMouse
  (bind _directhelmouselocationcache (Variables|Default|GetDirectHelMouseLocationCache))
  (Variables|Default|SetbShowMouseCursor true)
  (Class|PlayerController|SetMouseLocation (Math|Float|Truncate (.x _directhelmouselocationcache)) (Math|Float|Truncate (.y _directhelmouselocationcache))))