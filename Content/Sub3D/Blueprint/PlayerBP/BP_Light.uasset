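; BP_Light is an interactable light actor that can be carried in the left hand of whoever interacts with it.
; Its SpotLight is deactivated on BeginPlay and toggled through the StartLight and StopLight events.
; OnInteract snaps the actor to the interactor's hand_l socket only when IsHandled is already true, then sets it true again; otherwise it just prints a debug string.
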(event OnInteract(Interactable)
  (params (Interactor :type Sub%20Crew%20Character%20Object%20Reference))
  (if (Variables|Default|GetbIsHandled)
    (Development|PrintString "Hello")
    (Transformation|AttachActorToActor Interactor "hand_l" "SnapToTarget" "SnapToTarget" "KeepRelative" true)
    (Variables|Default|SetbIsHandled true)
    (else
      (Development|PrintString "XZ"))))

(event Custom|StopLight
  (Components|Activation|SetActive (Variables|Default|GetSpotLight) false false))

(event Custom|StartLight
  (Components|Activation|SetActive (Variables|Default|GetSpotLight) true false))

(event EventBeginPlay
  (Components|Activation|SetActive (Variables|Default|GetSpotLight) false false))

(event Collision|EventActorBeginOverlap
  (params (OtherActor :type Actor%20Object%20Reference)))

(event EventTick
  (params (DeltaSeconds :type Float%20%28single-precision%29)))

(fn ConstructionScript)