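; Helm station actor for a submarine, which players interact with to take or leave the station.
; Its interact event casts the interactor's controller to PC_SubPlayerController, then calls ServerExitStation if that controller is the current occupant, otherwise ServerEnterStation with itself.
; The Blueprint leaves the actual station handling to those controller calls; its view-target blend nodes for the occupant and submarine are disconnected and never run.
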(event OnInteract(Interactable)
  (params (Interactor :type Sub%20Crew%20Character%20Object%20Reference))
  (bind _aspc_sub_player_controller (Utilities|Casting|CastToPC_SubPlayerController (Pawn|GetController Interactor)))
  (if (== _aspc_sub_player_controller (Class|SubStationInterface|GetCurrentOccupant))
    (Class|SubPlayerController|ServerExitStation _aspc_sub_player_controller)
    (else
      (Class|SubPlayerController|ServerEnterStation _aspc_sub_player_controller self))))

(event EventBeginPlay)

(event Collision|EventActorBeginOverlap
  (params (OtherActor :type Actor%20Object%20Reference)))

(fn ConstructionScript)