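; BP_SubDoor_Exterior is an exterior submarine door that animates open and closed.
; OnDoorStateChanged routes to separate opening and closing events, each playing its own timeline to set DoorMesh's relative rotation.
; Opening drives pitch while closing drives yaw.
; Each event also toggles the DoorCollision component's active state, active when closed and inactive when open, without waiting for the animation to finish.
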(event Custom|ClosingDoor
  ;[0.15 0.15 0.15 0.5] DoorClose
  (Utilities|FlowControl|Sequence
    (:then_0
      (bind _rotation (Timeline|Timeline_0 Play)
        (:Update
          (Transformation|SetRelativeRotation (Variables|Default|GetDoorMesh) (Math|Rotator|MakeRotator 0.0 0.0 _rotation) false false))))
    (:then_1
      (Components|Activation|SetActive (Variables|Default|GetDoorCollision) true false))))

(event Custom|OpeningDoor
  (Utilities|FlowControl|Sequence
    (:then_0
      (bind _rotation (Timeline|Timeline Play)
        (:Update
          (Transformation|SetRelativeRotation (Variables|Default|GetDoorMesh) (Math|Rotator|MakeRotator 0.0 _rotation 0.0) false false))))
    (:then_1
      (Components|Activation|SetActive (Variables|Default|GetDoorCollision) false false))))

(event EventBeginPlay)

(event Collision|EventActorBeginOverlap
  (params (OtherActor :type Actor%20Object%20Reference)))

(event EventTick
  (params (DeltaSeconds :type Float%20%28single-precision%29)))

(event EventOnDoorStateChanged
  (params (bNowClosed :type Boolean))
  (if bNowClosed
    (CallFunction|ClosingDoor)
    (else
      (CallFunction|OpeningDoor))))

(fn ConstructionScript)