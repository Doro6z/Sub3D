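; Submarine door Blueprint that swings its mesh open or shut when the door state changes.
; OnDoorStateChanged takes a closed flag and snaps DoorMesh's relative rotation to zero when closed or to 90 degrees pitch when open, with no interpolation.
; It also activates the DoorCollision component on close and deactivates it on open, using SetActive rather than changing collision settings.
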(event Collision|EventActorBeginOverlap
  (params (OtherActor :type Actor%20Object%20Reference)))

(event EventOnDoorStateChanged
  (params (bNowClosed :type Boolean))
  (if bNowClosed
    ;[0.15 0.15 0.15 0.5] DoorClose
    (Utilities|FlowControl|Sequence
      (:then_0
        (Transformation|SetRelativeRotation (Variables|Default|GetDoorMesh) (Math|Rotator|MakeRotator 0.0 0.0 0.0) false false))
      (:then_1
        (Components|Activation|SetActive (Variables|Default|GetDoorCollision) true false)))
    (else
      ;[0.15 0.15 0.15 0.5] Door Open
      (Utilities|FlowControl|Sequence
        (:then_0
          (Transformation|SetRelativeRotation (Variables|Default|GetDoorMesh) (Math|Rotator|MakeRotator 0.0 9e+01 0.0) false false))
        (:then_1
          (Components|Activation|SetActive (Variables|Default|GetDoorCollision) false false))))))

(fn ConstructionScript)